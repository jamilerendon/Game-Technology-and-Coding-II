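; BP_Turret is an AI turret that tracks a sensed target and fires bullets at it.
; HandleSight sets or clears EnemyTarget from sight results and starts Attack when a target is seen.
; Tick rotates the Pivot toward a point slightly ahead of the target, using its velocity as lead.
; Attack spawns BP_Bullet at the spawn point, then re-calls itself after a RoundsPerMin-based delay while the target remains valid.
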(event Custom|Attack
  (Variables|Default|GetEnemyTarget ; Only shoot if we can see the \nplayer
    (:then
      (Game|SpawnActorfromClass "/Game/Blueprints/AI/BP_Bullet.BP_Bullet_C" (Transformation|GetWorldTransform (Variables|Default|GetBulletSpawnPoint)) "Undefined" "MultiplyWithRoot" 0 (Variables|Default|GetInitial%20Speed) self)
      (Utilities|FlowControl|Delay (/ 6e+01 (Variables|Default|GetRounds%20Per%20Min))) ; First Rate Calculation
      (CallFunction|Attack))
    (:else)))

(event EventBeginPlay)

(event Collision|EventActorBeginOverlap
  (params (OtherActor :type Actor%20Object%20Reference)))

(event EventTick
  (params (DeltaSeconds :type Float%20%28single-precision%29))
  (bind _enemytarget (Variables|Default|GetEnemyTarget))
  (Variables|Default|GetEnemyTarget
    (:then
      (Transformation|SetWorldRotation (Variables|Default|GetPivot) (Math|Rotator|FindLookatRotation (Transformation|GetWorldLocation (Variables|Default|GetDefaultSceneRoot)) (+ (Transformation|GetActorLocation _enemytarget) (* (Transformation|GetVelocity _enemytarget) 0.2))) false false))
    (:else)))

(event EventHandleSight
  (params (Target :type Actor%20Object%20Reference) (Successfully%20Sensed :type Boolean) (Location :type Vector :default "0, 0, 0"))
  (if Successfully%20Sensed ; Did we start or stop seeing \nthe player?
    (Variables|Default|SetEnemyTarget Target)
    (CallFunction|Attack)
    (else
      (Variables|Default|SetEnemyTarget 0) ; Clear the enemy target
    )))

(fn ConstructionScript)