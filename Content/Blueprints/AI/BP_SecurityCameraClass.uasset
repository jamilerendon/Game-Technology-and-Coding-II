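; Security camera AI that raises an alarm when it spots the player and sends guards to the sighting.
; A sight event drives a Looking, Investigating, Alert state machine, with green, blue and red materials showing the state.
; A one-second delay confirms a sighting, then Alert re-calls itself every second while sight holds, sending all BP_DumDum actors to the target's location.
; Losing sight during Alert leaves the state unchanged.
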(event Custom|HandleSight
  (params (Successfully%20Sensed :type Boolean) (Target :type Actor%20Object%20Reference))
  (switch Utilities|FlowControl|Switch|SwitchonE_CamState (Variables|Default|GetCameraState) ; What state are we currently in?
    (:NewEnumerator0
      (CallFunction|Investigating (Variables|Default|GetCurrentlySeePlayer)))))

(event Custom|Investigating
  (params (Sensed :type Boolean))
  (if Sensed ; Are we acquiring the target?
    (Variables|Default|SetCameraState "NewEnumerator1")
    (Rendering|Material|SetMaterial (Variables|Default|GetStaticMesh) 0 "/Niagara/DefaultAssets/GeometryCache/M_DefaultGeometryCacheMaterial_Blue.M_DefaultGeometryCacheMaterial_Blue")
    (Utilities|FlowControl|Delay 1.0)
    (if (Variables|Default|GetCurrentlySeePlayer)
      (CallFunction|Alert)
      (else
        (Variables|Default|SetCameraState "NewEnumerator0")))))

(event Custom|Alert
  (if (Variables|Default|GetCurrentlySeePlayer)
    (Variables|Default|SetCameraState "NewEnumerator2")
    (Rendering|Material|SetMaterial (Variables|Default|GetStaticMesh) 0 "/Niagara/DefaultAssets/GeometryCache/M_DefaultGeometryCacheMaterial_Red.M_DefaultGeometryCacheMaterial_Red")
    (bind _outactors (Actor|GetAllActorsOfClass "/Game/Blueprints/AI/BP_DumDum.BP_DumDum_C"))
    (for _array_element _outactors
      (Default|GotoSeePoint _array_element (Transformation|GetActorLocation (stale Custom|HandleSight Target))))
    (Utilities|FlowControl|Delay 1.0)
    (CallFunction|Alert)
    (else
      (CallFunction|Investigating false))))

(event Custom|Looking
  (Variables|Default|SetCameraState "NewEnumerator0")
  (Rendering|Material|SetMaterial (Variables|Default|GetStaticMesh) 0 "/Niagara/DefaultAssets/GeometryCache/M_DefaultGeometryCacheMaterial_Green.M_DefaultGeometryCacheMaterial_Green"))

(event EventBeginPlay)

(event Collision|EventActorBeginOverlap
  (params (OtherActor :type Actor%20Object%20Reference)))

(event EventTick
  (params (DeltaSeconds :type Float%20%28single-precision%29))
  (if (Variables|Default|GetCurrentlySeePlayer)
    (Development|PrintText "Seeing player" true true "(R=0.000000,G=0.660000,B=1.000000,A=1.000000)" 0.0)
    (else
      (Development|PrintText "NOT seeing player" true true "(R=0.000000,G=0.660000,B=1.000000,A=1.000000)" 0.0))))

(fn ConstructionScript)