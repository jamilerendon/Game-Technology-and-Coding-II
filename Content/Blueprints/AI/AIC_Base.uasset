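; Base AI controller that relays sight perception events to the pawn it controls.
; It stores the pawn on possess and listens for AI Perception target updates, skipping actors tagged "None".
; Stimuli are routed by sense class display name, with only sight handled.
; HandleSight passes the target and sensed state to the pawn's HandleSightMessage, with a zero location instead of the stimulus location.
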(event OnTargetPerceptionUpdated(AIPerception)
  (params (Actor :type Actor%20Object%20Reference) (Stimulus :type AI%20Stimulus%20Structure))
  (if (not (Actor|ActorHasTag Actor "None"))
    (bind _returnvalue (Class|AIPerceptionSystem|GetSenseClassforStimulus Stimulus))
    (switch string (Utilities|GetClassDisplayName _returnvalue)
      (:AISense_Sight
        (CallFunction|HandleSight (.bSuccessfullySensed (Utilities|Struct|BreakAIStimulus Stimulus)) Actor)))))

(event EventBeginPlay)

(event EventTick
  (params (DeltaSeconds :type Float%20%28single-precision%29)))

(event EventPossess
  (params (PossessedPawn :type Pawn%20Object%20Reference))
  (Variables|Default|SetPossessed%20Pawn PossessedPawn))

(fn ConstructionScript)

(fn HandleSight
  (params (Successfully%20Sensed :type Boolean) (Target%20Actor :type Actor%20Object%20Reference))
  (Class|BPIPerciever|HandleSight(Message) (Variables|Default|GetPossessed%20Pawn) Target%20Actor Successfully%20Sensed "0, 0, 0"))