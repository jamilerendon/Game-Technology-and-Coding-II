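; Health pickup actor that can be picked up, dropped or used to add to the first-person character's health pickup count.
; BeginPlay caches the player; Use increments that count, calls UpdateHealthPickups and plays a click sound.
; A Box trigger shows a widget when the player enters and hides it when any overlap ends.
; Pickup disables Health component collision and returns the item type; Drop restores collision and physics, then launches it forward.
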(event OnComponentEndOverlap(Box)
  (params (OverlappedComponent :type Primitive%20Component%20Object%20Reference) (OtherActor :type Actor%20Object%20Reference) (OtherComp :type Primitive%20Component%20Object%20Reference) (OtherBodyIndex :type Integer))
  (if true
    (Rendering|SetVisibility (Variables|Default|GetWidget) false false)))

(event OnComponentBeginOverlap(Box)
  (params (OverlappedComponent :type Primitive%20Component%20Object%20Reference) (OtherActor :type Actor%20Object%20Reference) (OtherComp :type Primitive%20Component%20Object%20Reference) (OtherBodyIndex :type Integer) (bFromSweep :type Boolean) (SweepResult :type Hit%20Result%20Structure%20%28by%20ref%29))
  (if (== OtherActor (Variables|Default|GetAs%20BP%20First%20Person%20Character))
    (Rendering|SetVisibility (Variables|Default|GetWidget) true false)))

(event EventBeginPlay
  (bind _asbp_first_person_character (Utilities|Casting|CastToBP_FirstPersonCharacter (Game|GetPlayerCharacter 0)))
  (Variables|Default|SetAs%20BP%20First%20Person%20Character _asbp_first_person_character))

(event Collision|EventActorBeginOverlap
  (params (OtherActor :type Actor%20Object%20Reference)))

(event EventDrop
  (bind _health (Variables|Default|GetHealth))
  (Collision|SetCollisionEnabled (Variables|Default|GetHealth) "QueryAndPhysics")
  (Physics|SetSimulatePhysics _health true)
  (Physics|AddImpulse _health (* (Math|Vector|GetForwardVector _health) 1e+03) "None" true))

(event EventTick
  (params (DeltaSeconds :type Float%20%28single-precision%29)))

(event EventUse
  (bind _as_bp_first_person_character (Variables|Default|GetAs%20BP%20First%20Person%20Character))
  (bind _result (Math|Integer|IncrementInt (Variables|/Game/FirstPerson/Blueprints/BP_FirstPersonCharacter.BP_FirstPersonCharacter_C|GetHealthPickups _as_bp_first_person_character))
    (:%20%20
      (Variables|/Game/FirstPerson/Blueprints/BP_FirstPersonCharacter.BP_FirstPersonCharacter_C|SetHealthPickups _as_bp_first_person_character _result)
      (Default|UpdateHealthPickups _as_bp_first_person_character)
      (Audio|PlaySoundatLocation "/Engine/VREditor/Sounds/VR_click3.VR_click3" (Transformation|GetActorLocation) "0, 0, 0" 1.0 1.0 0.0 0 0 0 0))))

(fn ConstructionScript)

(fn Pickup
  (params (Owner :type BPC%20Interact%20Object%20Reference%20%28by%20ref%29))
  (Collision|SetCollisionEnabled (Variables|Default|GetHealth) "NoCollision") ; Stop the key from pushing the player off the map
  (return (Variables|Default|GetItem%20Type)))