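; BPC_Inventory is an inventory component that stores the item type held in each slot as an array of enums.
; GetSlot reads an array entry and resolves it through GetItemDetails, which scans DT_Items for the row with the matching EnumName.
; SetSlot writes a type at an index and fires OnSlotUpdated so the currently held item can swap when its slot changes.
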(event EventBeginPlay)

(event EventTick
  (params (DeltaSeconds :type Float%20%28single-precision%29)))

(fn GetItemDetails
  (params (Requested%20Item :type E_Item%20Enum :default "NewEnumerator0"))
  (bind _outrownames (DataTable|GetDataTableRowNames "/Game/Blueprints/DataTables/DT_Items.DT_Items"))
  (for _array_element _outrownames
    (bind _returnvalue (Utilities|GetDataTableRow "/Game/Blueprints/DataTables/DT_Items.DT_Items" _array_element)
      (:then
        (if (Utilities|Enum|Equal(Enum) (.EnumName (Utilities|Struct|BreakS_Item _returnvalue)) Requested%20Item)
          (return _returnvalue))))))

(fn GetSlot
  (params (Item%20Type :type Integer))
  (bind _item_details (CallFunction|GetItemDetails (Utilities|Array|Get(acopy) (Variables|Default|GetEnumInv) Item%20Type)))
  (return _item_details))

(fn SetSlot
  (params (Item%20Type :type E_Item%20Enum :default "NewEnumerator3") (Index :type Integer))
  (Utilities|Array|SetArrayElem (Variables|Default|GetEnumInv) Index Item%20Type)
  (Default|CallOnSlotUpdated Index) ; If the slot we're currently looking at\ngets updated, it will swap to the new\nthing we're holding.
)