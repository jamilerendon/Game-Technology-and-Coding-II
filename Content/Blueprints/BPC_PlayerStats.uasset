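; Player stats component that tracks health, stamina and experience and displays them on a W_PlayerStats widget created at BeginPlay.
; Each stat is a vector of min, max and current, with Change and Set functions for health and experience that update their bars.
; Stamina only sets its bar at startup.
; When ChangeHealth detects depleted health, a one-shot death event fades the camera to red, then reloads the current level.
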(event Custom|PlayerHasDied
  (Utilities|FlowControl|DoOnce false
    (:Completed
      (CameraFades|StartCameraFade (Game|GetPlayerCameraManager 0) 0.0 1.0 1.0 "(R=1.000000,G=0.038004,B=0.000000,A=1.000000)" false true)
      (Utilities|FlowControl|Delay 2.0)
      (bind _returnvalue (Game|GetCurrentLevelName true))
      (Game|OpenLevel(byName) (Utilities|String|StringToName _returnvalue)))))

(event EventBeginPlay
  (bind _health (Variables|Default|GetHealth))
  (Utilities|FlowControl|Sequence
    (:then_0
      (bind _returnvalue (UserInterface|CreateWidget "/Game/UI/W_PlayerStats.W_PlayerStats_C"))
      (bind _output_get (Variables|Default|SetStatsWidget _returnvalue))
      (UserInterface|Viewport|AddtoViewport _output_get 0))
    (:then_1
      (CallFunction|SetHealth (.x _health) (.y _health) (.z _health))
      (Progress|SetPercent (Variables|/Game/UI/W_PlayerStats.W_PlayerStats_C|GetStaminaBar (Variables|Default|GetStatsWidget)) (.z (Variables|Default|GetStamina)))
      (Progress|SetPercent (Variables|/Game/UI/W_PlayerStats.W_PlayerStats_C|GetExperienceBar (Variables|Default|GetStatsWidget)) (.z (Variables|Default|GetExperience))))))

(event EventTick
  (params (DeltaSeconds :type Float%20%28single-precision%29)))

(fn ChangeHealth
  (params (By%20%20Amount :type Float%20%28double-precision%29))
  (Variables|Default|SetHealth (Math|Vector|MakeVector (.x (Variables|Default|GetHealth)) (.y (Variables|Default|GetHealth)) (+ (.z (Variables|Default|GetHealth)) By%20%20Amount)))
  (Progress|SetPercent (Variables|/Game/UI/W_PlayerStats.W_PlayerStats_C|GetHealthBar (Variables|Default|GetStatsWidget)) (/ (.z (Variables|Default|GetHealth)) (- (.y (Variables|Default|GetHealth)) (.x (Variables|Default|GetHealth))))) ; 0 - 100 is easy just return health z.\nWhat if 25 - 150?
  (Development|PrintString (Utilities|String|ToString(Float) (/ (.z (Variables|Default|GetHealth)) (- (.y (Variables|Default|GetHealth)) (.x (Variables|Default|GetHealth))))) true true "(R=0.091796,G=1.000000,B=0.405421,A=1.000000)")
  (if (<= (+ (.z (Variables|Default|GetHealth)) By%20%20Amount) 0.0) ; Is the player dead?
    (Development|PrintText "Player has died")
    (CallFunction|PlayerHasDied)))

(fn SetHealth
  (params (Health%20X :type Float%20%28double-precision%29) (Health%20Y :type Float%20%28double-precision%29) (Health%20Z :type Float%20%28double-precision%29))
  ;[0.15 0.15 0.15 0.5] Setting the temp variables to health's current values.
  (LocalVariables|SetMin%20Health Health%20X)
  (LocalVariables|SetMax%20Health Health%20Y)
  (LocalVariables|SetCurrent%20Health Health%20Z)
  (if (!= Health%20X -1.0) ; Have we been given a different\nminimum health?
    (LocalVariables|SetMin%20Health Health%20X) ; If we have, store the new\nmin health
  )
  (if (!= Health%20Y -1.0) ; Have we been given a max\nnew health?
    (LocalVariables|SetMax%20Health Health%20Y) ; Store the new max health.
  )
  (if (!= Health%20Z -1.0) ; Have we been given a new \ncurrent health.
    (LocalVariables|SetCurrent%20Health Health%20Z) ; Stores the current health.
  )
  (Variables|Default|SetHealth (Math|Vector|MakeVector (LocalVariables|GetMin%20Health) (LocalVariables|GetMax%20Health) (LocalVariables|GetCurrent%20Health)))
  ;[0.15 0.15 0.15 0.5] Update the widget code.
  (Progress|SetPercent (Variables|/Game/UI/W_PlayerStats.W_PlayerStats_C|GetHealthBar (Variables|Default|GetStatsWidget)) (/ (.y (Variables|Default|GetHealth)) (- (.z (Variables|Default|GetHealth)) (.x (Variables|Default|GetHealth))))) ; 0 - 100 is easy just return health z.\nWhat if 25 - 150?
)

(fn ChangeExp
  (params (By%20Amount :type Float%20%28double-precision%29))
  (Variables|Default|SetExperience (Math|Vector|MakeVector (.x (Variables|Default|GetExperience)) (.y (Variables|Default|GetExperience)) (+ (.z (Variables|Default|GetExperience)) By%20Amount)))
  (Progress|SetPercent (Variables|/Game/UI/W_PlayerStats.W_PlayerStats_C|GetExperienceBar (Variables|Default|GetStatsWidget)) (/ (.z (Variables|Default|GetExperience)) (- (.y (Variables|Default|GetExperience)) (.x (Variables|Default|GetExperience)))))
  (if (<= (+ (.z (Variables|Default|GetExperience)) By%20Amount) 0.0)
    _))

(fn SetExp
  (params (Exp%20X :type Float%20%28double-precision%29) (Exp%20Y :type Float%20%28double-precision%29) (Exp%20Z :type Float%20%28double-precision%29))
  (LocalVariables|SetMin%20Exp Exp%20X)
  (LocalVariables|SetMax%20Exp Exp%20Y)
  (LocalVariables|SetCurrent%20Exp Exp%20Z)
  (if (!= Exp%20X 0.0)
    (LocalVariables|SetMin%20Exp Exp%20X))
  (if (!= Exp%20Y 0.0)
    (LocalVariables|SetMax%20Exp Exp%20Y))
  (if (!= Exp%20Z 0.0)
    (LocalVariables|SetCurrent%20Exp Exp%20Z))
  (Variables|Default|SetExperience (Math|Vector|MakeVector (LocalVariables|GetMin%20Exp) (LocalVariables|GetMax%20Exp) (LocalVariables|GetCurrent%20Exp)))
  (Progress|SetPercent (Variables|/Game/UI/W_PlayerStats.W_PlayerStats_C|GetExperienceBar (Variables|Default|GetStatsWidget)) (/ (.y (Variables|Default|GetExperience)) (- (.z (Variables|Default|GetExperience)) (.x (Variables|Default|GetExperience))))))