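; BP_Spawner is an actor that repeatedly spawns a configured class at its SpawnLocation.
; A self-calling timed loop starts shortly after BeginPlay, skips colliding spawns and prints on success, without checking Looping.
; When not Looping, a first-person character entering its Trigger calls AddActor on the GM_SaveLoad game mode's LevelState.
; A separate Activate event destroys the spawner.
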(event OnComponentBeginOverlap(Trigger)
  (params (OverlappedComponent :type Primitive%20Component%20Object%20Reference) (OtherActor :type Actor%20Object%20Reference) (OtherComp :type Primitive%20Component%20Object%20Reference) (OtherBodyIndex :type Integer) (bFromSweep :type Boolean) (SweepResult :type Hit%20Result%20Structure%20%28by%20ref%29))
  (if (not (Variables|Default|GetLooping)) ; If we are looping, don't do\nanything
    (Utilities|Casting|CastToBP_FirstPersonCharacter OtherActor)
    (bind _asgm_save_load (Utilities|Casting|CastToGM_SaveLoad (Game|GetGameMode)))
    (Default|AddActor (Variables|/Game/Blueprints/SavingAndLoading/GM_SaveLoad.GM_SaveLoad_C|GetLevelState _asgm_save_load))))

(event Custom|Spawn%20The%20Thing
  (bind _returnvalue (Game|SpawnActorfromClass (Variables|Default|GetClass) (Transformation|GetWorldTransform (Variables|Default|GetSpawnLocation)) "DontSpawnIfColliding" "MultiplyWithRoot" 0 0))
  (Utilities|IsValid _returnvalue
    (:Is%20Valid
      (Development|PrintText "Spawned The Thing"))
    (:Is%20Not%20Valid
      _))
  (Utilities|FlowControl|Delay 5.0)
  (CallFunction|SpawntheThing))

(event EventBeginPlay
  (Utilities|FlowControl|Delay 1.0)
  (CallFunction|SpawntheThing))

(event Collision|EventActorBeginOverlap
  (params (OtherActor :type Actor%20Object%20Reference)))

(event EventTick
  (params (DeltaSeconds :type Float%20%28single-precision%29)))

(event EventActivate
  (Actor|DestroyActor) ; If we aren't looping,\ndestroy ourselves.
)

(fn ConstructionScript)