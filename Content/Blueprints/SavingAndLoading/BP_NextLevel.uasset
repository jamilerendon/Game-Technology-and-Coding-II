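; BP_NextLevel is an overlap trigger that moves the player to the Destination level.
; When BP_FirstPersonCharacter overlaps it, the GM_SaveLoad game mode saves the belt and backpack inventories.
; The saved position is the current level's PlayerStart transform rather than the player's own, resetting their location for the level being left.
; It then deletes the level state and opens Destination by object reference.
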(event EventBeginPlay)

(event Collision|EventActorBeginOverlap
  (params (OtherActor :type Actor%20Object%20Reference))
  (bind _asbp_first_person_character (Utilities|Casting|CastToBP_FirstPersonCharacter OtherActor)) ; Was it the player that ran through us?
  (bind _asgm_save_load (Utilities|Casting|CastToGM_SaveLoad (Game|GetGameMode))) ; Gets the game mode
  (bind _returnvalue (Actor|GetActorOfClass "/Script/Engine.PlayerStart")) ; reset the player's saved location to player\nstart for the level we're leaving.
  (Default|Save _asgm_save_load (Variables|/Game/Blueprints/BPC_Inventory.BPC_Inventory_C|GetEnumInv (Variables|/Game/FirstPerson/Blueprints/BP_FirstPersonCharacter.BP_FirstPersonCharacter_C|GetBPC_Inv_Belt _asbp_first_person_character)) (Variables|/Game/Blueprints/BPC_Inventory.BPC_Inventory_C|GetEnumInv (Variables|/Game/FirstPerson/Blueprints/BP_FirstPersonCharacter.BP_FirstPersonCharacter_C|GetBPC_Inv_Backpack _asbp_first_person_character)) (Transformation|GetActorTransform _returnvalue)) ; Save the player values.
  (Default|DeleteLevelState _asgm_save_load)
  (Game|OpenLevel(byObjectReference) (Variables|Default|GetDestination)))

(event EventTick
  (params (DeltaSeconds :type Float%20%28single-precision%29)))

(fn ConstructionScript)