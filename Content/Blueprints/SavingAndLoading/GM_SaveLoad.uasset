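; GM_SaveLoad is a game mode that saves, loads and deletes player progress and per-level state.
; On BeginPlay it loads or creates SG_Player for belt and backpack inventories, and SG_LevelState for actor states and player transform.
; Level state uses its own slot, named by appending the level name, and a saved location at the origin is not applied.
; Save writes both objects, while either delete event reopens the current level.
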(event Custom|Load
  ;[0.15 0.15 0.15 0.5] File Management for Loading
  (Utilities|FlowControl|Sequence
    (:then_0
      (bind _returnvalue (SaveGame|DoesSaveGameExist (Variables|Default|GetSlot%20Name))) ; Does the game exist?
      (if _returnvalue
        (bind _returnvalue_2 (SaveGame|LoadGamefromSlot (Variables|Default|GetSlot%20Name)))
        (bind _assg_player (Utilities|Casting|CastToSG_Player _returnvalue_2))
        (Variables|Default|SetPlayerSave _assg_player) ; We have the linked Game Mode's\nPlayerSave with the "save to file"\nplayer save.
        (bind _asbp_first_person_character (Utilities|Casting|CastToBP_FirstPersonCharacter (Game|GetPlayerCharacter 0)))
        (Default|SetInventory (Variables|/Game/FirstPerson/Blueprints/BP_FirstPersonCharacter.BP_FirstPersonCharacter_C|GetBPC_Inv_Belt _asbp_first_person_character) (Variables|/Game/Blueprints/SavingAndLoading/SG_Player.SG_Player_C|GetBelt (Variables|Default|GetPlayerSave))) ; Loads the belt
        ;[0.15 0.15 0.15 0.5] Is there save data for the location?
        (Default|SetInventory (Variables|/Game/FirstPerson/Blueprints/BP_FirstPersonCharacter.BP_FirstPersonCharacter_C|GetBPC_Inv_Backpack _asbp_first_person_character) (Variables|/Game/Blueprints/SavingAndLoading/SG_Player.SG_Player_C|GetInventory (Variables|Default|GetPlayerSave))) ; Loads the player inventory
        (else
          (bind _returnvalue_3 (SaveGame|CreateSaveGameObject "/Game/Blueprints/SavingAndLoading/SG_Player.SG_Player_C"))
          (Variables|Default|SetPlayerSave _returnvalue_3))))
    (:then_1
      (CallFunction|LoadLevel))))

(event Custom|Save
  (params (Belt :type Array%20of%20E_Item%20Enums :default "NewEnumerator3") (Inventory :type Array%20of%20E_Item%20Enums :default "NewEnumerator3") (Last%20Position :type Transform))
  (bind _playersave (Variables|Default|GetPlayerSave))
  ;[0.15 0.15 0.15 0.5] File Management for Saving
  (Utilities|FlowControl|Sequence
    (:then_0
      (Variables|/Game/Blueprints/SavingAndLoading/SG_Player.SG_Player_C|SetBelt _playersave Belt)
      (Variables|/Game/Blueprints/SavingAndLoading/SG_Player.SG_Player_C|SetInventory _playersave Inventory)
      (bind _returnvalue (SaveGame|SaveGametoSlot (Variables|Default|GetPlayerSave) (Variables|Default|GetSlot%20Name)))
      (if _returnvalue
        (Development|PrintString "Game saved to slot")
        (else
          (Development|PrintText "Could not save game to slot"))))
    (:then_1
      (CallFunction|SaveLevelState))))

(event Custom|LoadLevel
  ;[0.15 0.15 0.15 0.5] Load Level
  (bind _returnvalue (Game|GetCurrentLevelName true))
  (bind _returnvalue_2 (SaveGame|DoesSaveGameExist (Utilities|String|Append (Variables|Default|GetSlot%20Name) "_" _returnvalue)))
  (if _returnvalue_2
    (bind _returnvalue_3 (SaveGame|LoadGamefromSlot (Utilities|String|Append (Variables|Default|GetSlot%20Name) "_" _returnvalue)))
    (bind _assg_level_state (Utilities|Casting|CastToSG_LevelState _returnvalue_3))
    (bind _output_get (Variables|Default|SetLevelState _assg_level_state))
    (Default|LoadActorStates _output_get)
    ;[0.15 0.15 0.15 0.5] Load the players location and rotation, if it has been saved. (Moved from Player Save to Level State).
    (bind _asbp_first_person_character (Utilities|Casting|CastToBP_FirstPersonCharacter (Game|GetPlayerCharacter 0)))
    (if (not (Class|KismetMathLibrary|EqualExactlyVectorVector (.Location (Math|Transform|BreakTransform (Variables|/Game/Blueprints/SavingAndLoading/SG_LevelState.SG_LevelState_C|GetSavedLocation (Variables|Default|GetLevelState)))) "0, 0, 0")) ; Is the lalst transform set to 0,0,0?\nIf so, do nothing
      (Transformation|SetWorldTransform (Variables|/Script/Engine.Character|GetCapsuleComponent _asbp_first_person_character) (Variables|/Game/Blueprints/SavingAndLoading/SG_LevelState.SG_LevelState_C|GetSavedLocation (Variables|Default|GetLevelState)) false false) ; Allows for the player to spawn in at the location.
      (Pawn|SetControlRotation (Game|GetPlayerController 0) (.Rotation (Math|Transform|BreakTransform (Variables|/Game/Blueprints/SavingAndLoading/SG_LevelState.SG_LevelState_C|GetSavedLocation (Variables|Default|GetLevelState))))))
    (else
      (bind _returnvalue_4 (SaveGame|CreateSaveGameObject "/Game/Blueprints/SavingAndLoading/SG_LevelState.SG_LevelState_C"))
      (Variables|Default|SetLevelState _returnvalue_4))))

(event Custom|SaveLevelState
  (Variables|/Game/Blueprints/SavingAndLoading/SG_LevelState.SG_LevelState_C|SetSavedLocation (Variables|Default|GetLevelState) (stale Custom|Save Last%20Position))
  (bind _returnvalue (Game|GetCurrentLevelName true))
  (SaveGame|SaveGametoSlot (Variables|Default|GetLevelState) (Utilities|String|Append (Variables|Default|GetSlot%20Name) "_" _returnvalue)))

(event Custom|Delete%20Save
  (SaveGame|DeleteGameinSlot (Variables|Default|GetSlot%20Name)) ; Delete player save
  (bind _returnvalue (Game|GetCurrentLevelName true))
  (SaveGame|DeleteGameinSlot (Utilities|String|Append (Variables|Default|GetSlot%20Name) "_" _returnvalue)) ; Delete level state
  (Game|OpenLevel(byName) (Utilities|String|StringToName _returnvalue)))

(event Custom|Delete%20Level%20State
  (bind _returnvalue (Game|GetCurrentLevelName true))
  (SaveGame|DeleteGameinSlot (Utilities|String|Append (Variables|Default|GetSlot%20Name) "_" _returnvalue)) ; Delete level state
  (Game|OpenLevel(byName) (Utilities|String|StringToName _returnvalue)))

(event EventBeginPlay
  (Development|PrintText "GM_SaveLoad is running" true true "(R=1.000000,G=0.966173,B=0.260483,A=1.000000)") ; Tells us that the GM_SaveLoad is running\nproperly
  (CallFunction|Load))

(event EventTick
  (params (DeltaSeconds :type Float%20%28single-precision%29)))

(fn ConstructionScript)