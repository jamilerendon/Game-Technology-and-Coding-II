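; BP_ShopKeeper is a shopkeeper actor that opens a shop menu when the first-person character comes near.
; BeginPlay creates a W_ShopKeepMenu widget once, passing in the shopkeeper's BPCInventory.
; Sphere overlap adds the menu to the viewport and calls ShowInventory on the player.
; Leaving the sphere removes only the shop menu; a leftover inventory debug print is unconnected.
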(event OnComponentBeginOverlap(Sphere)
  (params (OverlappedComponent :type Primitive%20Component%20Object%20Reference) (OtherActor :type Actor%20Object%20Reference) (OtherComp :type Primitive%20Component%20Object%20Reference) (OtherBodyIndex :type Integer) (bFromSweep :type Boolean) (SweepResult :type Hit%20Result%20Structure%20%28by%20ref%29))
  (bind _asbp_first_person_character (Utilities|Casting|CastToBP_FirstPersonCharacter OtherActor))
  (UserInterface|Viewport|AddtoViewport (stale EventBeginPlay _returnvalue) 0)
  (Default|ShowInventory _asbp_first_person_character))

(event OnComponentEndOverlap(Sphere)
  (params (OverlappedComponent :type Primitive%20Component%20Object%20Reference) (OtherActor :type Actor%20Object%20Reference) (OtherComp :type Primitive%20Component%20Object%20Reference) (OtherBodyIndex :type Integer))
  (Utilities|Casting|CastToBP_FirstPersonCharacter OtherActor)
  (Widget|RemovefromParent (stale EventBeginPlay _returnvalue)))

(event EventBeginPlay
  (bind _returnvalue (UserInterface|CreateWidget "/Game/UI/W_ShopKeepMenu.W_ShopKeepMenu_C" 0 0 (Variables|Default|GetBPC_Inventory))))

(event Collision|EventActorBeginOverlap
  (params (OtherActor :type Actor%20Object%20Reference)))

(event EventTick
  (params (DeltaSeconds :type Float%20%28single-precision%29)))

(fn ConstructionScript)