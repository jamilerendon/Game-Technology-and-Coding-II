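; AI controller for BP_RangedEnemyAI that runs its behavior tree, with the first-person character as blackboard target.
; Sight perception switches the blackboard state, changes walk speed and starts or stops a looping fire timer.
; Perception updates are not filtered by actor, so any sighted actor triggers this.
; Firing only draws a debug line trace from gun to player; hits have no effect yet.
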(event OnPerceptionUpdated(AIPerception)
  (params (UpdatedActors :type Array%20of%20Actor%20Object%20References))
  (for _array_element UpdatedActors
    (bind _info (Class|AIPerceptionComponent|GetActorsPerception (Variables|Default|GetAIPerception) _array_element))
    (for _array_element_2 (.LastSensedStimuli (Utilities|Struct|BreakActorPerceptionBlueprintInfo _info))
      (bind _returnvalue (Class|AIPerceptionSystem|GetSenseClassforStimulus _array_element_2))
      (if (== _returnvalue "/Script/AIModule.AISense_Sight")
        (if (.bSuccessfullySensed (Utilities|Struct|BreakAIStimulus _array_element_2))
          (Development|PrintString "Player has been seen")
          (CallFunction|UpdateState "NewEnumerator1")
          (Default|SetWalkSpeed (Variables|Default|GetRanged%20Enemy%20AI) 3e+02)
          (CallFunction|StartFiring)
          (else
            (Development|PrintString "Player sight has been lost")
            (CallFunction|UpdateState "NewEnumerator0")
            (Default|SetWalkSpeed (Variables|Default|GetRanged%20Enemy%20AI) 1.5e+02)
            (CallFunction|StopFiring)))))))

(event Custom|Start%20Firing
  (bind _returnvalue (Utilities|Time|SetTimerbyEvent (delegate Custom|Fire) 0.1 true))
  (Variables|Default|SetFireTimerHandle _returnvalue))

(event Custom|Fire
  (bind _returnvalue (Collision|LineTraceByChannel (Transformation|GetWorldLocation (Variables|/Game/Blueprints/Enemies/BP_RangedEnemyAI.BP_RangedEnemyAI_C|GetGun (Variables|Default|GetRanged%20Enemy%20AI))) (Transformation|GetActorLocation (Variables|Default|GetPlayer)) "TraceTypeQuery2" false (Utilities|Array|MakeArray self) "ForDuration"))
  (if _returnvalue
    _))

(event Custom|Stop%20Firing
  (Utilities|Time|ClearandInvalidateTimerbyHandle (Variables|Default|GetFireTimerHandle)))

(event EventBeginPlay)

(event EventTick
  (params (DeltaSeconds :type Float%20%28single-precision%29)))

(event EventPossess
  (params (PossessedPawn :type Pawn%20Object%20Reference))
  (bind _asbp_ranged_enemy_ai (Utilities|Casting|CastToBP_RangedEnemyAI PossessedPawn))
  (Variables|Default|SetRanged%20Enemy%20AI _asbp_ranged_enemy_ai)
  (Utilities|FlowControl|Delay 0.2)
  (bind _returnvalue (Actor|GetActorOfClass "/Game/FirstPerson/Blueprints/BP_FirstPersonCharacter.BP_FirstPersonCharacter_C"))
  (Variables|Default|SetPlayer _returnvalue)
  (AI|RunBehaviorTree "/Game/Blueprints/Enemies/BT_RangedEnemyAI.BT_RangedEnemyAI")
  (AI|Components|Blackboard|SetValueasObject (AI|GetBlackboard 0) (Variables|Default|GetTarget%20Key%20Name) (Variables|Default|GetPlayer))
  (CallFunction|UpdateState "NewEnumerator0"))

(fn ConstructionScript)

(fn UpdateState
  (params (State :type E_RangedEnemyStatees%20Enum :default "NewEnumerator0"))
  (bind _output_get (Variables|Default|SetState State))
  (AI|Components|Blackboard|SetValueasEnum (AI|GetBlackboard 0) (Variables|Default|GetState%20Key%20Name) _output_get))